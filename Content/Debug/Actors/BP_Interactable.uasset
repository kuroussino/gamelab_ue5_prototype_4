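; BP_Interactable is an actor that highlights its static mesh when the player character is nearby.
; Every Tick, CheckOutline compares the distance to the player against OutlineActivationDistance and toggles Render Custom Depth, presumably for an outline effect.
; Enabling it at or within range requires the player to cast to BP_MainCharacter.
; A CheckLookAt gate on the character exists but is disconnected, so only distance controls the highlight.
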(event EventBeginPlay)

(event Collision|EventActorBeginOverlap
  (params (OtherActor :type Actor%20Object%20Reference)))

(event EventTick
  (params (DeltaSeconds :type Float%20%28single-precision%29))
  (CallFunction|CheckOutline))

(fn ConstructionScript)

(fn CheckOutline
  (bind _returnvalue (Game|GetPlayerCharacter 0))
  (Math|Float|CompareFloat (Transformation|GetDistanceTo _returnvalue) (Variables|Default|GetoutlineActivationDistance)
    (:>
      (Rendering|SetRenderCustomDepth (Variables|Default|GetStaticMesh) false))
    (:==
      (bind _asbp_main_character (Utilities|Casting|CastToBP_MainCharacter _returnvalue :!label _label))
      (Rendering|SetRenderCustomDepth (Variables|Default|GetStaticMesh) true))
    (:<
      (goto _label))))